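; BP_Bullet is a projectile actor that flies forward and explodes on hitting an opposing Player or Enemy actor.
; Tick moves it along its forward vector at Speed without sweeping, so hits rely on overlap events.
; On overlap, it ignores its owner and compares owner and target tags to allow only cross-team hits.
; A valid hit spawns an explosion effect and sound, then destroys the bullet after a short delay, applying no damage itself.
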(event `self.ReceiveActorBeginOverlap`
  (params (OtherActor :type "Actor Object Reference"))
  (bind _tags (`Actor.Tags` OtherActor))
  (bind _tags_2 (`Actor.Tags` (`self.GetOwner`)))
  (if (!= OtherActor (`self.GetOwner`))
    (if (or (and (`KismetArrayLibrary.Array_Contains` _tags "Player") (`KismetArrayLibrary.Array_Contains` _tags_2 "Enemy")) (and (`KismetArrayLibrary.Array_Contains` _tags_2 "Player") (`KismetArrayLibrary.Array_Contains` _tags "Enemy")))
      (`GameplayStatics.SpawnEmitterAtLocation` "/Game/StarterContent/Particles/P_Explosion.P_Explosion" (`self.K2_GetActorLocation`))
      (`GameplayStatics.PlaySound2D` "/Game/StarterContent/Audio/Explosion01.Explosion01" 1.0 1.0 0.0 null null)
      (`KismetSystemLibrary.Delay` 0.2)
      (`self.K2_DestroyActor`))))

(event `self.ReceiveTick`
  (params (DeltaSeconds :type "Float (single-precision)"))
  (`self.K2_SetActorLocation` (+ (* (`self.GetActorForwardVector`) DeltaSeconds (`self.Speed`)) (`self.K2_GetActorLocation`))))

(fn `UserConstructionScript`)