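; Player character for a space shooter that moves with Enhanced Input, fires ammo from its main cannon and tracks health.
; Firing is rate-limited by a timer, and Tick clamps the capsule inside fixed X/Y play bounds.
; Hits cost health with a brief invulnerability delay, while HealActor restores it up to a cap.
; At zero health it notifies the B_GM_Shooter game mode, explodes and destroys itself.
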(event `self.ReceiveBeginPlay`
  (bind _asplayer_controller (cast `PlayerController` (`self.GetController`)))
  (bind _returnvalue (pcsubsystem `EnhancedInputLocalPlayerSubsystem` _asplayer_controller))
  (`/Engine/EditorBlueprintResources/StandardMacros.IsValid` _returnvalue
    (:`Is Valid`
      (`EnhancedInputSubsystemInterface.AddMappingContext` _returnvalue "/Game/Inputs/BP_InputMapping.BP_InputMapping" 0 (struct)))))

(event `self.ReceiveActorBeginOverlap`
  (params (OtherActor :type "Actor Object Reference"))
  (cast `Pawn` OtherActor)
  (`GameplayStatics.SpawnEmitterAtLocation` null))

(event `EnhancedInput|/Game/Inputs/BP_InputFire`
  (params (ActionValue :type Boolean) (ElapsedSeconds :type "Float (double-precision)") (TriggeredSeconds :type "Float (double-precision)") (InputAction :type "InputAction Object Reference" :default "/Game/Inputs/BP_InputFire.BP_InputFire"))
  (:`Triggered`
    (if (`self.CanFire`)
      (`self.DoFire`)
      (set `self.CanFire` false)
      (`KismetSystemLibrary.K2_SetTimerDelegate` (delegate `UpdateFire`) (`self.FireDelay`)))))

(event `EnhancedInput|/Game/Inputs/BP_InputMove`
  (params (ActionValue :type "Vector2D Structure") (ElapsedSeconds :type "Float (double-precision)") (TriggeredSeconds :type "Float (double-precision)") (InputAction :type "InputAction Object Reference" :default "/Game/Inputs/BP_InputMove.BP_InputMove"))
  (:`Triggered`
    (`self.AddMovementInput` (+ (* (`self.GetActorRightVector`) ActionValue_X) (* ActionValue_Y (`self.GetActorForwardVector`))))))

(event `UpdateFire`
  (set `self.CanFire` true))

(event `HealActor`
  (set `self.Health` (`KismetMathLibrary.Clamp` (+ (`self.Health`) 1) 0 3)))

(event `DamageActor`
  (bind _output_get (set `self.Health` (- (`self.Health`) 1)))
  (if (== _output_get 0)
    (bind _asb_gm_shooter (cast `/Game/Blueprints/B_GM_Shooter` (`GameplayStatics.GetGameMode`)))
    (`/Game/Blueprints/B_GM_Shooter.PlayerDeath` _asb_gm_shooter)
    (`GameplayStatics.SpawnEmitterAtLocation` "/Game/StarterContent/Particles/P_Explosion.P_Explosion" (`SceneComponent.K2_GetComponentLocation` (`self.CapsuleComponent`)))
    (`self.K2_DestroyActor`)))

(event `self.ReceiveTick`
  (params (DeltaSeconds :type "Float (single-precision)"))
  (bind _capsulecomponent (`self.CapsuleComponent`))
  (bind (_returnvalue_x _returnvalue_y _returnvalue_z) (`KismetMathLibrary.BreakVector` (`SceneComponent.K2_GetComponentLocation` _capsulecomponent)))
  (`SceneComponent.K2_SetWorldLocation` _capsulecomponent (`KismetMathLibrary.MakeVector` (`KismetMathLibrary.FClamp` _returnvalue_x -750.0 750.0) (`KismetMathLibrary.FClamp` _returnvalue_y -1400.0 1400.0) _returnvalue_z) false false))

(event `/Game/Blueprints/BP_IHittable.Hit`
  (if (`self.CanBeHit`)
    (set `self.CanBeHit` false)
    (`self.DamageActor`)
    (`KismetSystemLibrary.Delay` 1.0)
    (set `self.CanBeHit` true)))

(fn `DoFire`
  (`|SpawnActorFromClass` (`self.Ammo`) (`SceneComponent.K2_GetComponentToWorld` (`self.MainCannon`)) "Undefined" "MultiplyWithRoot" self null))

(fn `UserConstructionScript`)