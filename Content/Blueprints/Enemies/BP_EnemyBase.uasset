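; Base enemy for a shooter that flies along its spawn forward vector and destroys itself past a negative X limit, checked after each volley.
; Tick accumulates time to fire Ammo tagged "Enemy" from every child of Cannons.
; Player overlap or Hit calls the OnEnemyDestroy dispatcher and notifies B_GM_Shooter.
; The bound Destroyed handler has an even chance to spawn BP_PowerUp, then destroys the actor after a short delay.
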(event `self.ReceiveActorBeginOverlap`
  (params (OtherActor :type "Actor Object Reference"))
  (if (`KismetArrayLibrary.Array_Contains` (`Actor.Tags` OtherActor) "Player")
    (`self.OnEnemyDestroy`)
    (bind _asb_gm_shooter (cast `/Game/Blueprints/B_GM_Shooter` (`GameplayStatics.GetGameMode`)))
    (`/Game/Blueprints/B_GM_Shooter.EnemyDestroyed` _asb_gm_shooter)))

(event `self.ReceiveBeginPlay`
  (set `self.MovementVector` (`self.GetActorForwardVector`))
  (add `self.OnEnemyDestroy` (delegate `Destroyed`)))

(event `Destroyed`
  (`|ExecutionSequence`
    (:`then_0`
      (if (< (`KismetMathLibrary.RandomFloat`) 0.5)
        (`|SpawnActorFromClass` "/Game/Blueprints/BP_PowerUp.BP_PowerUp_C" (`SceneComponent.K2_GetComponentToWorld` (`self.Arrow`)) "Undefined" "MultiplyWithRoot" null null)))
    (:`then_1`
      (`KismetSystemLibrary.Delay` 0.2)
      (`self.K2_DestroyActor`))))

(event `self.ReceiveTick`
  (params (DeltaSeconds :type "Float (single-precision)"))
  (`self.Move` DeltaSeconds)
  (bind _output_get (set `self.ShotCurrentTime` (+ DeltaSeconds (`self.ShotCurrentTime`))))
  (if (> _output_get (`self.DelayShoot`))
    (set `self.ShotCurrentTime` 0.0)
    (`self.Fire`)
    (if (< (.x (`SceneComponent.K2_GetComponentLocation` (`self.Root`))) -900.0)
      (`self.K2_DestroyActor`))))

(event `OnActorBeginOverlap_Event`
  (params (OverlappedActor :type "Actor Object Reference") (OtherActor :type "Actor Object Reference")))

(event `/Game/Blueprints/BP_IHittable.Hit`
  (`self.OnEnemyDestroy`)
  (bind _asb_gm_shooter (cast `/Game/Blueprints/B_GM_Shooter` (`GameplayStatics.GetGameMode`)))
  (`/Game/Blueprints/B_GM_Shooter.EnemyDestroyed` _asb_gm_shooter))

(fn `Fire`
  (locals (NewLocalVar :type "Array of SceneComponent Object Reference"))
  (for _array_element (`SceneComponent.GetChildrenComponents` (`self.Cannons`) false)
    (bind _returnvalue (`|SpawnActorFromClass` (`self.Ammo`) (`SceneComponent.K2_GetComponentToWorld` _array_element) "Undefined" "MultiplyWithRoot" self null))
    (`self.K2_SetActorRotation` _returnvalue (`self.K2_GetActorRotation`) false)
    (`KismetArrayLibrary.Array_Add` (`Actor.Tags` _returnvalue) "Enemy")))

(fn `Move`
  (params (Delta :type "Float (single-precision)"))
  (`self.K2_SetActorLocation` (+ (* (`self.MovementVector`) Delta (`self.Speed`)) (`self.K2_GetActorLocation`))))

(fn `UserConstructionScript`)