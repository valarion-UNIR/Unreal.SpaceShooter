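; BP_Enemy2 is an enemy variant that sets a diagonal, zigzag heading through the MovementVector variable.
; BeginPlay starts the heading as forward plus right, relative to the actor.
; Tick checks the root's world Y against symmetric limits and flips the sideways component when one is crossed, keeping the forward component.
; The file only sets the vector and contains no code that applies the movement.
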(event `self.ReceiveBeginPlay`
  (`parent.ReceiveBeginPlay`)
  (set `self.MovementVector` (+ (`self.GetActorRightVector`) (`self.GetActorForwardVector`))))

(event `self.ReceiveTick`
  (params (DeltaSeconds :type "Float (single-precision)"))
  (bind (_returnvalue_x _returnvalue_y) (`KismetMathLibrary.BreakVector` (`SceneComponent.K2_GetComponentLocation` (`self.Root`))))
  (`parent.ReceiveTick` DeltaSeconds)
  (if (> _returnvalue_y 1400.0)
    (set `self.MovementVector` (+ (`self.GetActorRightVector`) (`self.GetActorForwardVector`)))
    (elif (< _returnvalue_y -1400.0)
      (set `self.MovementVector` (+ (- (0.0 0.0 0.0) (`self.GetActorRightVector`)) (`self.GetActorForwardVector`))))))

(fn `UserConstructionScript`
  (`parent.UserConstructionScript`))