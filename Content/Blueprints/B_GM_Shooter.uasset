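; B_GM_Shooter is the shooter's game mode, tracking progress and destroyed enemies and relaying player death to the HUD.
; Tick adds Increment to Progress every frame without scaling by delta time.
; PlayerDeath forwards to BP_Hud on player controller 0, while EnemyDestroyed increments the DestroyedEnemies counter.
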(event `self.ReceiveTick`
  (params (DeltaSeconds :type "Float (single-precision)"))
  ;[1 1 1] Update progress
  (set `self.Progress` (+ (`self.Progress`) (`self.Increment`))))

(event `PlayerDeath`
  ;[1 1 1] Propagate player death to HUD
  (bind _asbp_hud (cast `/Game/Blueprints/UI/BP_Hud` (`PlayerController.GetHUD` (`GameplayStatics.GetPlayerController` 0))))
  (`/Game/Blueprints/UI/BP_Hud.PlayerDeath` _asbp_hud))

(event `EnemyDestroyed`
  (set `self.DestroyedEnemies` (+ (`self.DestroyedEnemies`) 1)))

(fn `UserConstructionScript`)