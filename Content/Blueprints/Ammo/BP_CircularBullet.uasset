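; BP_CircularBullet is a bullet Blueprint whose Scene component spins to give it circular motion.
; The construction script uses Radius to offset the Capsule and Scene components along local X, setting up the orbit around a pivot.
; Each Tick, after the parent's logic, it yaws Scene by RotationPerSecond scaled by delta time, keeping the spin frame-rate independent.
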(event `self.ReceiveTick`
  (params (DeltaSeconds :type "Float (single-precision)"))
  (`parent.ReceiveTick` DeltaSeconds)
  (`SceneComponent.K2_AddRelativeRotation` (`self.Scene`) (`KismetMathLibrary.MakeRotator` 0.0 0.0 (* DeltaSeconds (`self.RotationPerSecond`))) false false))

(fn `UserConstructionScript`
  (`parent.UserConstructionScript`)
  (`SceneComponent.K2_SetRelativeLocation` (`self.Capsule`) (`KismetMathLibrary.MakeVector` (`self.Radius`)) false false)
  (bind _result (`/Engine/EditorBlueprintResources/StandardMacros.NegateFloat` (`self.Radius`))
    (:`  `
      (`SceneComponent.K2_SetRelativeLocation` (`self.Scene`) (`KismetMathLibrary.MakeVector` _result) false false))))