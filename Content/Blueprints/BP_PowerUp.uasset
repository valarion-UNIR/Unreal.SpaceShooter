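; BP_PowerUp is a drifting healing pickup for the space shooter.
; Each Tick moves it along its forward vector at Speed without sweeping, and destroys it once its absolute world X passes a fixed limit.
; Overlap with an actor tagged Player calls HealActor on BP_SpaceShooterCharacter, then destroys the pickup after a short delay.
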(event `self.ReceiveActorBeginOverlap`
  (params (OtherActor :type "Actor Object Reference"))
  (if (`KismetArrayLibrary.Array_Contains` (`Actor.Tags` OtherActor) "Player")
    (`|ExecutionSequence`
      (:`then_0`
        (bind _asbp_space_shooter_character (cast `/Game/Blueprints/BP_SpaceShooterCharacter` OtherActor))
        (`/Game/Blueprints/BP_SpaceShooterCharacter.HealActor` _asbp_space_shooter_character))
      (:`then_1`
        (`KismetSystemLibrary.Delay` 0.2)
        (`self.K2_DestroyActor`)))))

(event `self.ReceiveTick`
  (params (DeltaSeconds :type "Float (single-precision)"))
  (bind _returnvalue (+ (* (`self.GetActorForwardVector`) DeltaSeconds (`self.Speed`)) (`self.K2_GetActorLocation`)))
  (`self.K2_SetActorLocation` _returnvalue)
  (if (> (`KismetMathLibrary.Abs` (.x _returnvalue)) 900.0)
    (`self.K2_DestroyActor`)))

(fn `UserConstructionScript`)