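; Base enemy actor for a shooter that flies straight along its initial forward vector and fires at a fixed interval.
; Tick moves it by Speed without sweep and accumulates time until DelayShoot, then spawns Ammo at the Scene component, aligned to the actor's rotation.
; Overlapping a Player-tagged actor calls the OnEnemyDestroy dispatcher, whose bound handler destroys it after a short delay, and notifies B_GM_Shooter.
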(event `self.ReceiveActorBeginOverlap`
  (params (OtherActor :type "Actor Object Reference"))
  (if (`KismetArrayLibrary.Array_Contains` (`Actor.Tags` OtherActor) "Player")
    (`self.OnEnemyDestroy`)
    (bind _asb_gm_shooter (cast `/Game/Blueprints/B_GM_Shooter` (`GameplayStatics.GetGameMode`)))
    (`/Game/Blueprints/B_GM_Shooter.EnemyDestroyed` _asb_gm_shooter)))

(event `self.ReceiveBeginPlay`
  (set `self.MovementVector` (`self.GetActorForwardVector`))
  (add `self.OnEnemyDestroy` (delegate `Destroyed`)))

(event `Destroyed`
  (`KismetSystemLibrary.Delay` 0.2)
  (`self.K2_DestroyActor`))

(event `self.ReceiveTick`
  (params (DeltaSeconds :type "Float (single-precision)"))
  (`self.Move` DeltaSeconds)
  (bind _output_get (set `self.ShotCurrentTime` (+ DeltaSeconds (`self.ShotCurrentTime`))))
  (if (> _output_get (`self.DelayShoot`))
    (set `self.ShotCurrentTime` 0.0)
    (`self.Fire`)))

(event `OnActorBeginOverlap_Event`
  (params (OverlappedActor :type "Actor Object Reference") (OtherActor :type "Actor Object Reference")))

(fn `Fire`
  (bind _returnvalue (`|SpawnActorFromClass` (`self.Ammo`) (`SceneComponent.K2_GetComponentToWorld` (`self.Scene`)) "Undefined" "MultiplyWithRoot" self null))
  (`self.K2_SetActorRotation` _returnvalue (`self.K2_GetActorRotation`) false))

(fn `Move`
  (params (B :type "Float (single-precision)"))
  (`self.K2_SetActorLocation` (+ (* (`self.MovementVector`) B (`self.Speed`)) (`self.K2_GetActorLocation`))))

(fn `UserConstructionScript`)